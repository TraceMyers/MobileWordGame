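; Background graphics actor that endlessly scrolls a set of cube meshes, apparently as purple stripes.
; On BeginPlay it caches each cube's angled teleport offset from the bottom plane and a speed, higher for smaller cubes and those farther from Visplane, floored at half the maximum.
; Tick moves each cube along its local X axis.
; Overlapping the bottom plane teleports a cube to the top plane plus its cached offset, looping the motion.
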(event OnComponentBeginOverlap(bot_plane)
  (params (OverlappedComponent :type Primitive%20Component%20Object%20Reference) (OtherActor :type Actor%20Object%20Reference) (OtherComp :type Primitive%20Component%20Object%20Reference) (OtherBodyIndex :type Integer) (bFromSweep :type Boolean) (SweepResult :type Hit%20Result%20Structure%20%28by%20ref%29))
  (bind _asstatic_mesh_component (Utilities|Casting|CastToStaticMeshComponent OtherComp))
  (Transformation|SetWorldLocation _asstatic_mesh_component (+ (Utilities|Array|Get(acopy) (Variables|Default|Getteleport_offsets) (.Value (Utilities|Map|Find (Variables|Default|Getmesh_to_index) _asstatic_mesh_component))) (Transformation|GetWorldLocation (Variables|Default|Gettop_plane))) false false))

(event EventBeginPlay
  (bind _output_get (Variables|Default|Setcubes (Utilities|Array|MakeArray (Variables|Default|GetCube17) (Variables|Default|GetCube11) (Variables|Default|GetCube12) (Variables|Default|GetCube13) (Variables|Default|GetCube8) (Variables|Default|GetCube16) (Variables|Default|GetCube2) (Variables|Default|GetCube7) (Variables|Default|GetCube15) (Variables|Default|GetCube18) (Variables|Default|GetCube6) (Variables|Default|GetCube10) (Variables|Default|GetCube9) (Variables|Default|GetCube5) (Variables|Default|GetCube3) (Variables|Default|GetCube4) (Variables|Default|GetCube) (Variables|Default|GetCube1) (Variables|Default|GetCube14) (Variables|Default|GetCube25) (Variables|Default|GetCube23) (Variables|Default|GetCube24) (Variables|Default|GetCube19) (Variables|Default|GetCube20) (Variables|Default|GetCube22) (Variables|Default|GetCube21))))
  (for (_array_element _array_index) _output_get
    (Utilities|Map|Add (Variables|Default|Getmesh_to_index) _array_element _array_index)
    (Utilities|Array|Add (Variables|Default|Getsphere_radii) (.SphereRadius (Collision|GetComponentBounds _array_element)))
    (Utilities|Array|Add (Variables|Default|Getsphere_plane_dists) (Math|Vector|Distance(Vector) (.Origin (Collision|GetComponentBounds (Variables|Default|Getvisplane))) (.Origin (Collision|GetComponentBounds _array_element))))
    (bind _returnvalue (Class|BGGrafixInst|AngledTeleportOffset (Variables|Default|Getbot_plane) _array_element (== _array_index 0)))
    (Utilities|Array|Add (Variables|Default|Getteleport_offsets) _returnvalue))
  (Variables|Default|Setmax_plane_dist (.MaxValue (Math|Float|MaxOfFloatArray (Variables|Default|Getsphere_plane_dists))))
  (Variables|Default|Setmax_radius (.MaxValue (Math|Float|MaxOfFloatArray (Variables|Default|Getsphere_radii))))
  (for (_array_element_2 _array_index_2) (Variables|Default|Getsphere_radii)
    (if (< (+ (* (- 1.0 (/ _array_element_2 (Variables|Default|Getmax_radius))) 0.5) (* (/ (Utilities|Array|Get(acopy) (Variables|Default|Getsphere_plane_dists) _array_index_2) (Variables|Default|Getmax_plane_dist)) 0.5)) 0.5)
      (Utilities|Array|Add (Variables|Default|Getsphere_speeds) (* (Math|Float|MakeLiteralFloat 0.5) (Variables|Default|Getsphere_max_speed)))
      (else
        (Utilities|Array|Add (Variables|Default|Getsphere_speeds) (* (+ (* (- 1.0 (/ _array_element_2 (Variables|Default|Getmax_radius))) 0.5) (* (/ (Utilities|Array|Get(acopy) (Variables|Default|Getsphere_plane_dists) _array_index_2) (Variables|Default|Getmax_plane_dist)) 0.5)) (Variables|Default|Getsphere_max_speed)))))))

(event Collision|EventActorBeginOverlap
  (params (OtherActor :type Actor%20Object%20Reference)))

(event EventTick
  (params (DeltaSeconds :type Float%20%28single-precision%29))
  (for (_array_element _array_index) (Variables|Default|Getcubes)
    (Class|KismetMathLibrary|VectorSet (Variables|Default|Getmove_vec) (* (Utilities|Array|Get(acopy) (Variables|Default|Getsphere_speeds) _array_index) DeltaSeconds) 0.0 0.0)
    (Transformation|AddLocalOffset _array_element (Variables|Default|Getmove_vec) false false)))

(fn ConstructionScript)